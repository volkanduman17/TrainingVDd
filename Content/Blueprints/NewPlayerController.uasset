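; Player controller that shows the level/HP widget and lets number keys switch possession between the third-person character, the master ship and the hover bike.
; Choosing a vehicle possesses the first one found in the world, destroys the cached character and updates the Gemide/Hoverda state flags.
; Returning to foot respawns the character at the current pawn's location if needed.
; F prints the controlled pawn for debugging.
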(event `self.ReceiveBeginPlay`
  (bind _returnvalue (`|CreateWidget` "/Game/Level_HP_Widget.Level_HP_Widget_C"))
  (`UserWidget.AddToViewport` _returnvalue 0)
  (bind _asbp_third_person_character (cast `/Game/ThirdPerson/Blueprints/BP_ThirdPersonCharacter` (`GameplayStatics.GetPlayerPawn` 0)))
  (`/Engine/EditorBlueprintResources/StandardMacros.IsValid` _asbp_third_person_character
    (:`Is Valid`
      (set `self.TPC` _asbp_third_person_character))))

(event `Key|F`
  (params (Key :type "Key Structure"))
  (:`Pressed`
    (`KismetSystemLibrary.PrintString` (`KismetStringLibrary.Conv_ObjectToString` (`self.K2_GetPawn`)))))

(event `Key|One`
  (params (Key :type "Key Structure"))
  ;[1 1 1] Pawn Geçişleri
  (:`Pressed`
    (set `self.Gemide?` false)
    (set `self.Hoverda?` false)
    (`/Engine/EditorBlueprintResources/StandardMacros.IsValid` (`self.TPC`)
      (:`Is Valid`
        _)
      (:`Is Not Valid`
        (bind _returnvalue (`|SpawnActorFromClass` "/Game/ThirdPerson/Blueprints/BP_ThirdPersonCharacter.BP_ThirdPersonCharacter_C" (`KismetMathLibrary.MakeTransform` (`self.K2_GetActorLocation` (`self.K2_GetPawn`))) "AdjustIfPossibleButAlwaysSpawn" "MultiplyWithRoot" null null))
        (bind _output_get (set `self.TPC` _returnvalue))))
    (`self.Possess` _output_get)))

(event `Key|Two`
  (params (Key :type "Key Structure"))
  (bind _tpc (`self.TPC`))
  ;[1 1 1] Pawn Geçişleri
  (:`Pressed`
    (set `self.Gemide?` true)
    (set `self.Hoverda?` false)
    (bind _outactors (`GameplayStatics.GetAllActorsOfClass` "/Game/Q1_MasterShip.Q1_MasterShip_C"))
    (bind _output_get (set `self.GemiRef` (`|GetArrayItem` _outactors)))
    (`self.Possess` _output_get)
    (`/Engine/EditorBlueprintResources/StandardMacros.IsValid` _tpc
      (:`Is Valid`
        (`self.K2_DestroyActor` _tpc)
        (set `self.TPC` null)))))

(event `Key|Three`
  (params (Key :type "Key Structure"))
  (bind _tpc (`self.TPC`))
  ;[1 1 1] Pawn Geçişleri
  (:`Pressed`
    (set `self.Gemide?` false)
    (set `self.Hoverda?` true)
    (bind _returnvalue (`GameplayStatics.GetActorOfClass` "/Game/Q1_HoverBike.Q1_HoverBike_C"))
    (`self.Possess` (`GameplayStatics.GetPlayerController` 0) _returnvalue)
    (`/Engine/EditorBlueprintResources/StandardMacros.IsValid` _tpc
      (:`Is Valid`
        (`self.K2_DestroyActor` _tpc)
        (set `self.TPC` null)))))

(fn `UserConstructionScript`)